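; BP_Dyson_CineCamera is a cine camera Blueprint that moves its camera component to preset transforms.
; The CameraTransformMove event converts its parameter to a row name and looks up the target in DT_CameraTransform.
; A Timeline eases the world transform toward that target with CircularIn, blending from the current transform on each update rather than a cached start.
; Debug prints report the target during the move and announce completion.
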(event Custom|CameraTransformMove
  (params (NewParam :type String))
  (bind _returnvalue (Utilities|GetDataTableRow "/Game/Yun/Data/DT_CameraTransform.DT_CameraTransform" (Utilities|String|StringToName NewParam))
    (:then
      (bind _새_트랙_0 (Timeline|timeline PlayFromStart)
        (:Update
          (Transformation|SetWorldTransform (Variables|CameraActor|GetCameraComponent) (Math|Interpolation|Ease "CircularIn" _새_트랙_0 (Transformation|GetWorldTransform (Variables|CameraActor|GetCameraComponent)) (Utilities|Struct|BreakST_CameraTransform _returnvalue)) false false)
          (Development|PrintString (Utilities|String|ToString(Transform) (Utilities|Struct|BreakST_CameraTransform _returnvalue))))
        (:Finished
          (Development|PrintString "ChangeFinished" true true "(R=0.254749,G=1.000000,B=0.000000,A=1.000000)" 1e+01))))))

(event EventBeginPlay)

(event Collision|EventActorBeginOverlap
  (params (OtherActor :type Actor%20Object%20Reference)))

(event EventTick
  (params (DeltaSeconds :type Float%20%28single-precision%29)))

(fn ConstructionScript)